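; Lobby game mode that registers joining players, shares lobby state and server-travels to the selected arena map.
; PostLogin reads server settings from the game instance, sets up each LobbyPC and spawns a default 0_Base pawn at a random spawn point.
; Map changes and roster updates are pushed to every controller, and CanWeStart stays false while any player still has the default character.
; Kick-list and character-swap events are empty stubs.
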(event Custom|SwapCharacter
  (params (Player :type Player%20Controller%20Object%20Reference) (CharacterClass :type Character%20Class%20Reference) (Changed%20Status :type Boolean)))

(event Custom|EvreyoneUpdate
  (bind _allplayercontrollers (Variables|서버세팅|GetAllPlayerControllers))
  ;[1 1 1] 호출시 접속자 들에게 로비 정보 업데이트
  (bind _output_get (Variables|서버세팅|SetCurrentPlayers (Utilities|Array|Length (Variables|서버세팅|GetAllPlayerControllers))))
  (if (> _output_get 0)
    (Utilities|Array|Clear (Variables|서버세팅|GetConnectedPlayers))
    (for _array_element _allplayercontrollers
      (bind _aslobby_pc (Utilities|Casting|CastToLobbyPC _array_element))
      (Utilities|Array|Add (Variables|서버세팅|GetConnectedPlayers) (Variables|/Game/BluePrints/Lobby/LobbyPC.LobbyPC_C|GetPlayerSetting _aslobby_pc))
      (Default|UpdateNumberOfPlayers _aslobby_pc (Variables|서버세팅|GetCurrentPlayers) (Variables|서버세팅|GetMaxPlayers)))
    (for _array_element_2 _allplayercontrollers
      (bind _aslobby_pc_2 (Utilities|Casting|CastToLobbyPC _array_element_2))
      (Default|AddPlayerInfo _aslobby_pc_2 (Variables|서버세팅|GetConnectedPlayers))
      (Default|UpdateAvailableCharavters _aslobby_pc_2 (Variables|서버세팅|GetAvailableCharacters))
      (CallFunction|AddtoKickList))
    (bind _array_element_3 (Utilities|Array|ForEachLoopwithBreak (Variables|서버세팅|GetConnectedPlayers))
      (:LoopBody
        (if (== (.MyPlayerCharacter (Utilities|Struct|BreakPlayerInfo _array_element_3)) "/Game/BluePrints/Charactors/0_Base.0_Base_C")
          (Variables|서버세팅|SetCanWeStart? false)
          (CallFunction|CannotStartGame)
          (else
            (Variables|서버세팅|SetCanWeStart? true)))))))

(event Custom|launchThe%20game
  (bind _returnvalue (Game|GetPlayerController 0))
  ;[1 1 1] 게임 설정으로 결정한 맵에서 실행
  (switch int (Variables|서버세팅|GetGM_MapID)
    (:0
      (Development|ExecuteConsoleCommand "servertravel/Game/Maps/Arena01" _returnvalue))
    (:1
      (Development|ExecuteConsoleCommand "servertravel/Game/Maps/Arena02" _returnvalue))))

(event Custom|RespawnPlayers
  (params (PlayerController :type Player%20Controller%20Object%20Reference))
  (bind _returnvalue (Pawn|GetControlledPawn PlayerController))
  (bind _spawnpoints (Variables|서버세팅|GetSpawnPoints))
  ;[1 1 1] 로비에 입장하면 플레이어를 기본캐릭터로 스폰시킴 /나머지 플레이어들에게 로비를 업데이트하라고 통보
  (Utilities|IsValid _returnvalue
    (:Is%20Valid
      (Actor|DestroyActor _returnvalue))
    (:Is%20Not%20Valid
      _))
  (bind _returnvalue_2 (Game|SpawnActorfromClass "/Game/BluePrints/Charactors/0_Base.0_Base_C" (Transformation|GetActorTransform (Utilities|Array|Get(acopy) _spawnpoints (Math|Random|RandomIntegerinRange 0 (- (Utilities|Array|Length _spawnpoints) 1)))) "Undefined" 0 0))
  (Pawn|Possess PlayerController _returnvalue_2)
  (CallFunction|EvreyoneUpdate))

(event Custom|AddToKickList)

(event Custom|CannotStartGame
  ;[1 1 1] 호출시 접속자 들에게 로비 정보 업데이트
  (Utilities|Array|ForEachLoopwithBreak (Variables|서버세팅|GetConnectedPlayers)) ; enters at Break
)

(event Custom|ServerupdateGamesetting
  (params (MapImage :type Texture%202D%20Object%20Reference) (MapName :type Text) (MapTime :type Text) (MapID :type Integer))
  ;[1 1 1] 서버에 변동사항이 생기면 각 클라리언트에게 로비정보를 업데이트하라고 알림
  (Variables|서버세팅|SetGM_MapImage MapImage)
  (Variables|서버세팅|SetGM_MapName MapName)
  (Variables|서버세팅|SetGM_MapTime MapTime)
  (Variables|서버세팅|SetGM_MapID MapID)
  (for _array_element (Variables|서버세팅|GetAllPlayerControllers)
    (bind _aslobby_pc (Utilities|Casting|CastToLobbyPC _array_element))
    (Default|UPdateLobbySettings _aslobby_pc (Variables|서버세팅|GetGM_MapImage) (Variables|서버세팅|GetGM_MapName) (Variables|서버세팅|GetGM_MapTime))))

(event EventPostLogin
  (params (NewPlayer :type Player%20Controller%20Object%20Reference))
  ;[1 1 1] 로그인 이후 이벤트를 발동하는 초기 구성 단계 - 플레이어 컨트롤러에서 로비를 구성하고 플레이어를 스폰시킴
  (Networking|SwitchHasAuthority
    (:Authority
      (Utilities|Array|Add (Variables|서버세팅|GetAllPlayerControllers) NewPlayer)
      (bind _outactors (Actor|GetAllActorsOfClass 0))
      (Variables|서버세팅|SetSpawnPoints _outactors)
      (bind _asgame_info_instace (Utilities|Casting|CastToGameInfoInstace (Game|GetGameInstance)))
      (Variables|서버세팅|SetServerName (Variables|/Game/BluePrints/AllLevels/GameInfoInstace.GameInfoInstace_C|GetServerName _asgame_info_instace))
      (Variables|서버세팅|SetMaxPlayers (Variables|/Game/BluePrints/AllLevels/GameInfoInstace.GameInfoInstace_C|GetMaxPlayers _asgame_info_instace))
      (bind _aslobby_pc (Utilities|Casting|CastToLobbyPC NewPlayer))
      (Default|InitialSetup _aslobby_pc)
      (Default|SetupLobbyMenu _aslobby_pc (Variables|서버세팅|GetServerName))
      (Default|UPdateLobbySettings _aslobby_pc (Variables|서버세팅|GetGM_MapImage) (Variables|서버세팅|GetGM_MapName) (Variables|서버세팅|GetGM_MapTime))
      (CallFunction|RespawnPlayers _aslobby_pc))))

(fn ConstructionScript)